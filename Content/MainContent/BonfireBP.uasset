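; Interactable bonfire actor that lights up when used and acts as a save point for the world.
; Interact sets FireActive, writes the save through SSaveGameSubsystem, prints a confirmation, then calls UpdateFlames.
; UpdateFlames activates the particle system when FireActive is set, and OnActorLoaded calls it too so the flames match the loaded state.
; GetInteractText returns an empty prompt.
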(event `UpdateFlames`
  (if (`self.bFireActive`)
    (`ActorComponent.Activate` (`self.ParticleSystem`) false)))

(event `SGameplayInterface.Interact`
  (params (InstigatorPawn :type "Pawn Object Reference"))
  (set `self.bFireActive` true)
  (`SSaveGameSubsystem.WriteSaveGame` (subsystem `SSaveGameSubsystem`))
  (`KismetSystemLibrary.PrintString` "WORLD SAVED")
  (`self.UpdateFlames`))

(event `SGameplayInterface.OnActorLoaded`
  (`self.UpdateFlames`))

(fn `GetInteractText`
  (params (InstigatorPawn :type "Pawn Object Reference"))
  (returns (ReturnValue :type Text))
  (return ""))

(fn `UserConstructionScript`)